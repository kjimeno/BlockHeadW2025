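; BP_SpeedBoost is a pickup that temporarily boosts the player's speed.
; On BeginPlay it caches the player pawn and that pawn's current ForwardForce as the default.
; Any overlap with its mesh sets the player's ForwardForce to BoostForce and hides the mesh, without checking the overlapping actor.
; After BoostDuration it restores the cached force and destroys itself.
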(event OnComponentBeginOverlap(SpeedBoostMesh)
  (params (OverlappedComponent :type Primitive%20Component%20Object%20Reference) (OtherActor :type Actor%20Object%20Reference) (OtherComp :type Primitive%20Component%20Object%20Reference) (OtherBodyIndex :type Integer) (bFromSweep :type Boolean) (SweepResult :type Hit%20Result%20Structure%20%28by%20ref%29))
  ;[0.03119 1 0.1322 0.5] On Begin Overlap:
  ;;[0.03119 1 0.1322 0.5] Turn Visibility Off and Boost the Player's Speed
  (Variables|/Game/BlockHead/Core/Actors/BP_Player.BP_Player_C|SetForwardForce (Variables|Default|GetPlayer) (Variables|Default|GetBoostForce))
  (Rendering|SetVisibility (Variables|Default|GetSpeedBoostMesh) false false)
  (Utilities|FlowControl|Delay (Variables|Default|GetBoostDuration))
  ;;[0.03119 1 0.1322 0.5] Destroy Speed Boost and Reset Player's Speed
  (Variables|/Game/BlockHead/Core/Actors/BP_Player.BP_Player_C|SetForwardForce (Variables|Default|GetPlayer) (Variables|Default|GetDefaultForwardForce))
  (Actor|DestroyActor))

(event EventBeginPlay
  ;[0.03119 1 0.1322 0.5] Begin Play: Save a Reference to the Player and the Forward Force
  (bind _asbp_player (Utilities|Casting|CastToBP_Player (Game|Player|GetPlayerPawn 0)))
  (bind _output_get (Variables|Default|SetPlayer _asbp_player))
  (Variables|Default|SetDefaultForwardForce (Variables|/Game/BlockHead/Core/Actors/BP_Player.BP_Player_C|GetForwardForce _output_get)))

(fn ConstructionScript)